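; GM_MusicBox is a game mode for a music box scene with an on-screen piano.
; On BeginPlay it focuses the game viewport, shows the mouse cursor, then creates the Piano widget, adds it to the viewport and gives it user focus.
; A SetKeyPitch event copies the game mode's PitchArray into the piano widget.
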(event `self.ReceiveBeginPlay`
  (bind _returnvalue (`GameplayStatics.GetPlayerController` 0))
  (`WidgetBlueprintLibrary.SetFocusToGameViewport`)
  (set `PlayerController.bShowMouseCursor` true _returnvalue)
  (bind _returnvalue_2 (`|CreateWidget` "/Game/UMG/Piano.Piano_C"))
  (bind _output_get (set `self.PianoKeys` _returnvalue_2))
  (`UserWidget.AddToViewport` _output_get 0)
  (`Widget.SetUserFocus` _output_get _returnvalue))

(event `SetKeyPitch`
  (set `/Game/UMG/Piano.PitchArray` (`self.PitchArray`) (`self.PianoKeys`)))

(fn `UserConstructionScript`)